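; BP_Download is a Blueprint that, despite its name, uploads images from given file paths and reports the outcome.
; EventUploadImage passes the paths to UploadImage with success and failure callbacks.
; Success stores the returned hash, prints it and calls CallOnUploadSuccess.
; Failure prints the error code and message, then calls CallOnUploadFailed.
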(event Custom|EventUploadImage
  (params (ImagePaths :type Array%20of%20Strings))
  (Class|BFLDownloader|UploadImage ImagePaths (delegate Custom|API_Upload_Success) (delegate Custom|API_UploadFailed)))

(event Custom|API_Upload_Success
  (params (Hash :type String))
  ;[1 1 1] 성공
  (bind _output_get (Variables|Default|SetHash Hash))
  (Development|PrintText (Utilities|Text|FormatText "Hash: {Hash}" _output_get))
  (Default|CallOnUploadSuccess))

(event Custom|API_UploadFailed
  (params (ErrorCode :type EHttpErrorCode%20Enum :default "None") (ErrorMessage :type String))
  ;[1 1 1] 실패
  (Development|PrintText (Utilities|Text|FormatText "result: {Code} / message: {Message}" (Utilities|String|EnumtoString ErrorCode) ErrorMessage))
  (Default|CallOnUploadFailed))

(fn ConstructionScript)