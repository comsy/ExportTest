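; BP_Relight sends image relighting requests to an API through RelightImage, using stored key, source, result and lighting image paths plus lighting strength and rotation angles.
; EventRelightWithValue overrides strength, theta and phi, then joins the same request path as EventRelight.
; Success and failure callbacks print the outcome and call CallOnRequestSuccess or CallOnRequestFailed to report it.
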(event Custom|API_Success
  (params (bSuccess :type Boolean) (ResultPath :type String))
  (Development|PrintText (Utilities|Text|FormatText "result: {success} / path: {path}" bSuccess ResultPath))
  (Default|CallOnRequestSuccess))

(event Custom|API_Failed
  (params (ErrorCode :type EHttpErrorCode%20Enum :default "None") (ErrorMessage :type String))
  (Development|PrintText (Utilities|Text|FormatText "result: {Code} / path: {Message}" (Utilities|String|EnumtoString ErrorCode) ErrorMessage))
  (Default|CallOnRequestFailed))

(event Custom|EventRelight
  (Development|PrintText "요청시작")
  (Class|BFLRelightRequester|RelightImage (Variables|Authentication|GetApiKey) (Variables|Path|GetSourceImagePath) (Variables|Path|GetResultImagePath) (Variables|Path|GetLightingImagePath) (Variables|POST|GetLightingStrength) (Variables|POST|GetLightingRotationTheta) (Variables|POST|GetLightingRotationPhi) (Variables|POST|GetAutoKey) (Variables|POST|GetPreview) (delegate Custom|API_Success) (delegate Custom|API_Failed))
  (Development|PrintText "요청완료"))

(event Custom|EventRelightWithValue
  (params (LightingStrength :type Float%20%28double-precision%29) (LightingRotationTheta :type Integer) (LightingRotationPhi :type Integer))
  (Variables|POST|SetLightingStrength LightingStrength)
  (Variables|POST|SetLightingRotationTheta LightingRotationTheta)
  (Variables|POST|SetLightingRotationPhi LightingRotationPhi)
  (Development|PrintText "요청시작")
  (Class|BFLRelightRequester|RelightImage (Variables|Authentication|GetApiKey) (Variables|Path|GetSourceImagePath) (Variables|Path|GetResultImagePath) (Variables|Path|GetLightingImagePath) (Variables|POST|GetLightingStrength) (Variables|POST|GetLightingRotationTheta) (Variables|POST|GetLightingRotationPhi) (Variables|POST|GetAutoKey) (Variables|POST|GetPreview) (delegate Custom|API_Success) (delegate Custom|API_Failed))
  (Development|PrintText "요청완료"))

(fn ConstructionScript)